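; Startup actor that shows the logo splash when the game begins, then opens the default start map.
; BeginPlay enables dynamic resolution, adds the logo widget through the QP UI subsystem and loads the main audio mix.
; A fixed Delay chain plays the logo fade-in, the init sound, then the same animation reversed as fade-out.
; Finally it reads the QP_DefaultStartMap setting from QP base data and opens that map.
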(event EventBeginPlay
  ;[1 1 1] 启动动态分辨率
  (bind _returnvalue (Settings|GetGameUserSettings))
  (Class|GameUserSettings|SetDynamicResolutionEnabled _returnvalue true)
  (Class|GameUserSettings|ApplyNonResolutionSettings _returnvalue)
  ;[1 1 1] 添加ui
  (bind _returnvalue_2 (Class|QPGIMUserInterface|QPAddUserInterfacebyClass (Subsystems|GetQPGIMUserInterface) "/QipaWorldUEPlugin/Widget/QP_WBP_LogoFadeIn.QP_WBP_LogoFadeIn_C" "None"))
  ;[1 1 1] 播放渐入动画
  (bind _aswbp_logo_fade_in (Utilities|Casting|CastToWBP_LogoFadeIn _returnvalue_2))
  (Utilities|FlowControl|Delay 0.3)
  ;[1 1 1] 加载音效
  (Class|AudioModulationStatics|LoadMixfromProfile "/QipaWorldUEPlugin/Blueprints/Sound/Control/QPCBM_Main.QPCBM_Main")
  (UserInterface|Animation|PlayAnimation _aswbp_logo_fade_in (Variables|/Game/QipaWorld3D/Widget/WBP_LogoFadeIn.WBP_LogoFadeIn_C|GetQP_LogoFadIn _aswbp_logo_fade_in) 0.0 1 "Forward" 1.0 false)
  ;[1 1 1] 播放音效
  (Utilities|FlowControl|Delay 1.0)
  (Class|QPGIMSound|QPPlay2DSoundbySound (Subsystems|GetQPGIMSound) "/QipaWorldUEPlugin/Blueprints/Sound/InitGame.InitGame")
  ;[1 1 1] 播放渐出动画
  (Utilities|FlowControl|Delay 1.0)
  (UserInterface|Animation|PlayAnimation _aswbp_logo_fade_in (Variables|/Game/QipaWorld3D/Widget/WBP_LogoFadeIn.WBP_LogoFadeIn_C|GetQP_LogoFadIn _aswbp_logo_fade_in) 0.0 1 "Reverse" 1.0 false)
  ;[1 1 1] 进入游戏
  (Utilities|FlowControl|Delay 1.0)
  (bind _returnvalue_3 (Class|QPGIMBaseData|QPGetDefaultSetting (Subsystems|GetQPGIMBaseData)))
  (bind _returnvalue_4 (Class|QPData|QPGetFString _returnvalue_3 "QP_DefaultStartMap"))
  (Class|QPGIMMap|QPOpenMap (Subsystems|GetQPGIMMap) _returnvalue_4))

(event Collision|EventActorBeginOverlap
  (params (OtherActor :type Actor%20Object%20Reference)))

(event EventTick
  (params (DeltaSeconds :type Float%20%28single-precision%29)))

(fn ConstructionScript)